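; BP_SNAPawn is the player pawn for ShootNAdapt, providing look and hitscan shooting with no movement logic in its graphs.
; Enhanced Input IA_Look drives controller yaw and pitch, while IA_Shoot calls Shoot on press and applies a fixed damage to the returned actor.
; Shoot line-traces from the eye viewpoint along its forward vector up to ShotRange, with debug drawing left on, and returns the hit actor.
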(event `EnhancedInput|/Game/ShootNAdapt/Player/Controls/InputActions/IA_Look`
  (params (ActionValue :type "Vector2D Structure") (ElapsedSeconds :type "Float (double-precision)") (TriggeredSeconds :type "Float (double-precision)") (InputAction :type "InputAction Object Reference" :default "/Game/ShootNAdapt/Player/Controls/InputActions/IA_Look.IA_Look"))
  (:`Triggered`
    (`self.AddControllerPitchInput` ActionValue_Y)
    (`self.AddControllerYawInput` ActionValue_X)))

(event `EnhancedInput|/Game/ShootNAdapt/Player/Controls/InputActions/IA_Shoot`
  (params (ActionValue :type Boolean) (ElapsedSeconds :type "Float (double-precision)") (TriggeredSeconds :type "Float (double-precision)") (InputAction :type "InputAction Object Reference" :default "/Game/ShootNAdapt/Player/Controls/InputActions/IA_Shoot.IA_Shoot"))
  (:`Started`
    (bind _hitactor (`self.Shoot`))
    (`GameplayStatics.ApplyDamage` _hitactor 1.0)))

(fn `Shoot`
  (returns (HitActor :type "Actor Object Reference"))
  (bind (_outlocation _outrotation) (`self.GetActorEyesViewPoint`))
  (bind _outhit (`KismetSystemLibrary.LineTraceSingle` :`Start` _outlocation :`End` (+ _outlocation (* (`KismetMathLibrary.Conv_RotatorToVector` _outrotation) (`self.ShotRange`))) :`TraceChannel` "TraceTypeQuery3" :`DrawDebugType` "ForDuration"))
  (return (`.HitActor` (`GameplayStatics.BreakHitResult` _outhit))))

(fn `UserConstructionScript`)