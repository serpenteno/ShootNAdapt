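; Game mode for a target-shooting game that adapts difficulty to player performance, driving menus and rounds.
; Each round spawns targets one at a time at random TargetPoints, chaining the next from the previous one's EndPlay.
; Hits and lifetimes yield score, accuracy and reaction time for the end screen.
; When connected, it posts stats to a local HTTP server, whose response sets target class and lifespan through difficulty lookup maps.
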(event `self.ReceiveBeginPlay`
  (bind _returnvalue (`GameplayStatics.GetPlayerController` 0))
  (bind _outactors (`GameplayStatics.GetAllActorsOfClass` "/Script/Engine.TargetPoint"))
  (set `self.TargetSpawnPoints` _outactors)
  (bind _asbp_snapawn (cast `/Game/ShootNAdapt/Player/BP_SNAPawn` (`GameplayStatics.GetPlayerPawn` 0)))
  (set `self.PlayerPawn` _asbp_snapawn)
  (`self.SetDifficultyLevels` (`self.DifficultyLevels`))
  (`GameplayStatics.PlaySound2D` (`self.Music`) 0.5 1.0 0.0 null null)
  (bind _returnvalue_2 (`|CreateWidget` "/Game/ShootNAdapt/W_MainMenu.W_MainMenu_C"))
  (`UserWidget.AddToViewport` _returnvalue_2 0)
  (`WidgetBlueprintLibrary.SetInputMode_UIOnlyEx` _returnvalue _returnvalue_2)
  (set `PlayerController.bShowMouseCursor` true _returnvalue)
  (set `self.InitialPlayerRotation` (`Controller.GetControlRotation` _returnvalue)))

(event `Event StartRound`
  (bind _returnvalue (`GameplayStatics.GetPlayerController` 0))
  (`/Engine/EditorBlueprintResources/StandardMacros.IsValid` (stale `Event EndRound` _returnvalue_2)
    (:`Is Valid`
      (`Widget.RemoveFromParent` (stale `Event EndRound` _returnvalue_2)))
    (:`Is Not Valid`
      _))
  (`self.ResetRoundStats`)
  (`Controller.SetControlRotation` (`GameplayStatics.GetPlayerController` 0) (`self.InitialPlayerRotation`))
  (bind _returnvalue_2 (`|CreateWidget` "/Game/ShootNAdapt/Round/UI/W_Round.W_Round_C"))
  (`UserWidget.AddToViewport` _returnvalue_2 0)
  (`self.OnStartRound` (`self.DifficultyLevels`))
  (bind _spawnedtarget (`self.SpawnTarget` :!label _label))
  (`/Engine/EditorBlueprintResources/StandardMacros.IsValid` _spawnedtarget
    (:`Is Valid`
      (add `self.OnEndPlay` _spawnedtarget (delegate `Event TargetEndPlay`))
      (add `/Game/ShootNAdapt/Targets/BP_Target.OnHit` _spawnedtarget (delegate `Event TargetHit`))
      (`WidgetBlueprintLibrary.SetInputMode_GameOnly` _returnvalue)
      (set `PlayerController.bShowMouseCursor` false _returnvalue))))

(event `Event TargetEndPlay` :!signature `self.OnEndPlay`
  (params (Actor :type "Actor Object Reference") (EndPlayReason :type "EEndPlayReason Enum" :default "Destroyed"))
  (set `self.TotalTargetsLifetime` (+ (`self.ComputeActorLifetime` Actor) (`self.TotalTargetsLifetime`)))
  (goto _label))

(event `Event TargetHit`
  (params (TargetValue :type Integer))
  (set `self.TotalScore` (+ TargetValue (`self.TotalScore`)))
  (`/Engine/EditorBlueprintResources/StandardMacros.IncrementInt` (`self.TotalHitTargetsNum`)
    (:`  `
      (`self.OnTotalScoreUpdated`))))

(event `Event EndRound`
  (bind _result (`self.ComputeAccuracy`))
  (bind _result_2 (`self.ComputeReactionTime`))
  (bind _returnvalue (`GameplayStatics.GetPlayerController` 0))
  (bind (_difficultysettings_targetclass _difficultysettings_targetlifespan) (break `/Game/ShootNAdapt/Round/DifficultyLevel/SDifficultySettings` (`self.DifficultySettings`)))
  (`Widget.RemoveFromParent` (stale `Event StartRound` _returnvalue_2))
  (bind _returnvalue_2 (`|CreateWidget` "/Game/ShootNAdapt/Round/UI/W_RoundEnd.W_RoundEnd_C"))
  (`UserWidget.AddToViewport` _returnvalue_2 0)
  (`self.OnEndRound` _result _result_2)
  (`WidgetBlueprintLibrary.SetInputMode_UIOnlyEx` _returnvalue _returnvalue_2)
  (set `PlayerController.bShowMouseCursor` true _returnvalue)
  (if (`self.bPlayerConnected`)
    (`self.Event SendPlayerStats` (make `/Game/ShootNAdapt/Player/SPlayerStats` _result (/ _result_2 _difficultysettings_targetlifespan)))))

(event `Event SendPlayerStats`
  (params (PlayerStats :type "/Game/ShootNAdapt/Player/SPlayerStats Structure"))
  (bind _outjsonstring (`|StructToJsonString` PlayerStats))
  (bind (_outheader _result_body) (`|HttpRequest` "127.0.0.1:8000/send_player_stats" "Post" (struct) _outjsonstring)
    (:`On Success`
      (bind _output_get (set `self.DifficultyLevels` _result_body))
      (`self.SetDifficultyLevels` _output_get))
    (:`On Error`
      (`KismetSystemLibrary.PrintString` "Error sending player stats. Connection has been propably lost." true false (struct :`R` 1.0 :`A` 1.0) 5.0)
      (set `self.bPlayerConnected` false)))
  (`self.OnHttpPostRequest`))

(fn `ComputeAccuracy`
  (returns (Result :type "Float (double-precision)"))
  (return (/ (`self.TotalHitTargetsNum`) (`KismetMathLibrary.Conv_IntToDouble` (`/Game/ShootNAdapt/Player/BP_SNAPawn.ShotsNum` (`self.PlayerPawn`))))))

(fn `ComputeActorLifetime`
  (params (Actor :type "Actor Object Reference"))
  (returns (Result :type "Float (double-precision)"))
  (return (- (`Actor.InitialLifeSpan` Actor) (`self.GetLifeSpan` Actor))))

(fn `ComputeReactionTime`
  (returns (Result :type "Float (double-precision)"))
  (return (/ (`self.TotalTargetsLifetime`) (`self.InitialTargetNum`))))

(fn `ResetRoundStats`
  (set `self.TotalScore` 0)
  (set `self.CurrentTargetNum` (`self.InitialTargetNum`))
  (set `self.TotalHitTargetsNum` 0)
  (set `self.TotalTargetsLifetime` 0.0))

(fn `SetDifficultyLevels`
  (params (DifficultyLevels :type "/Game/ShootNAdapt/Round/DifficultyLevel/SDifficultyLevels Structure"))
  (bind (_targetsize _targetlifespan) (break `/Game/ShootNAdapt/Round/DifficultyLevel/SDifficultyLevels` DifficultyLevels))
  (setmembers `/Game/ShootNAdapt/Round/DifficultyLevel/SDifficultySettings` :`StructRef` (`self.DifficultySettings`) :`TargetClass` (`BlueprintMapLibrary.Map_Find` (`self.DifficultyLevelToTargetClass`) _targetsize) :`TargetLifeSpan` (`BlueprintMapLibrary.Map_Find` (`self.DifficultyLevelToTargetLifeSpan`) _targetlifespan)))

(fn `SpawnTarget`
  (returns (SpawnedTarget :type "/Game/ShootNAdapt/Targets/BP_Target Object Reference"))
  (bind (_difficultysettings_targetclass _difficultysettings_targetlifespan) (break `/Game/ShootNAdapt/Round/DifficultyLevel/SDifficultySettings` (`self.DifficultySettings`)))
  (bind _currenttargetnum (`self.CurrentTargetNum`))
  (if (> _currenttargetnum 0)
    (`/Engine/EditorBlueprintResources/StandardMacros.DecrementInt` _currenttargetnum
      (:`  `
        (bind _returnvalue (`|SpawnActorFromClass` _difficultysettings_targetclass (`self.GetTransform` (`KismetArrayLibrary.Array_Random` (`self.TargetSpawnPoints`))) "AlwaysSpawn" "MultiplyWithRoot" null _difficultysettings_targetlifespan null))))
    (else
      (`self.Event EndRound`)))
  (return _returnvalue))

(fn `UserConstructionScript`)