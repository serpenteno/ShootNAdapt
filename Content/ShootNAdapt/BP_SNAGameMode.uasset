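; Game mode for the ShootNAdapt target-shooting round, which spawns targets, tracks the total score and swaps the round widget for the round-end widget.
; SpawnTarget places one timed-lifespan target at a random TargetPoint while the TargetNum countdown lasts, then ends the round.
; Each target's destruction event triggers the next spawn, chaining the round without a timer.
; Target hits add their value to TotalScore and broadcast the update.
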(event `self.ReceiveBeginPlay`
  (bind _outactors (`GameplayStatics.GetAllActorsOfClass` "/Script/Engine.TargetPoint"))
  (set `self.TargetSpawnPoints` _outactors)
  (`self.Event StartRound`))

(event `Event StartRound`
  (bind _returnvalue (`|CreateWidget` "/Game/ShootNAdapt/UI/W_Round.W_Round_C"))
  (`UserWidget.AddToViewport` _returnvalue 0)
  (bind _spawnedtarget (`self.SpawnTarget`))
  (`/Engine/EditorBlueprintResources/StandardMacros.IsValid` _spawnedtarget
    (:`Is Valid`
      (add `self.OnDestroyed` _spawnedtarget (delegate `Event TargetDestroyed`))
      (add `/Game/ShootNAdapt/Targets/BP_Target.OnHit` _spawnedtarget (delegate `Event TargetHit`)))))

(event `Event TargetDestroyed` :!signature `self.OnDestroyed`
  (params (DestroyedActor :type "Actor Object Reference"))
  (clear `self.OnDestroyed` DestroyedActor)
  (bind _spawnedtarget (`self.SpawnTarget`))
  (`/Engine/EditorBlueprintResources/StandardMacros.IsValid` _spawnedtarget
    (:`Is Valid`
      (add `self.OnDestroyed` _spawnedtarget (delegate `Event TargetDestroyed`))
      (add `/Game/ShootNAdapt/Targets/BP_Target.OnHit` _spawnedtarget (delegate `Event TargetHit`)))))

(event `Event TargetHit`
  (params (TargetValue :type Integer))
  (set `self.TotalScore` (+ TargetValue (`self.TotalScore`)))
  (`self.OnTotalScoreUpdated`))

(event `Event EndRound`
  (`Widget.RemoveFromParent` (stale `Event StartRound` _returnvalue))
  (bind _returnvalue (`|CreateWidget` "/Game/ShootNAdapt/UI/W_RoundEnd.W_RoundEnd_C"))
  (`UserWidget.AddToViewport` _returnvalue 0))

(fn `SpawnTarget`
  (returns (SpawnedTarget :type "/Game/ShootNAdapt/Targets/BP_Target Object Reference"))
  (if (> (`self.TargetNum`) 0)
    (`/Engine/EditorBlueprintResources/StandardMacros.DecrementInt` (`self.TargetNum`)
      (:`  `
        (bind _returnvalue (`|SpawnActorFromClass` (`self.TargetClass`) (`self.GetTransform` (`KismetArrayLibrary.Array_Random` (`self.TargetSpawnPoints`))) "AlwaysSpawn" "MultiplyWithRoot" null (`self.TargetLifeSpan`) null))))
    (else
      (`self.Event EndRound`)))
  (return _returnvalue))

(fn `UserConstructionScript`)